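; Wizard fireball gameplay ability that launches a projectile and applies an effect to targets around the location under the mouse.
; It captures the mouse hit location, faces it and plays a throw montage, spawning the projectile on the shoot AnimNotify gameplay event.
; A later StartTrace gameplay event triggers a target trace at the captured location, applies the effect and ends the ability.
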(event Ability|EventActivateAbility
  (bind _targetdata (|GetTargetDataUnderMouse)
    (:MouseTargetData
      (bind _output_get (Variables|Default|SetMouseHitLocation (.Location (Utilities|Struct|BreakTurpAbilityTargetData _targetdata))))
      (Class|TurpGameplayAbility|FaceTargetBeforeAttacking _output_get)
      (|PlayMontageandWaitProxy "None" "/Game/Assets/Animations/AM_MagicThrow03.AM_MagicThrow03" 1.0 "None" true 1.0 0.0 false
        (:then
          ;[1 0.3431 0.9228] Wait for AnimNotify on Montage
          (Ability|Tasks|WaitGameplayEvent "(TagName=\"AnimNotify.Shoot\")" 0 true
            (:EventReceived
              (Class|ProjectileAbility|SpawnProjectile)
              (Ability|Tasks|WaitGameplayEvent "(TagName=\"GameplayEvent.StartTrace\")" 0 true
                (:EventReceived
                  (Class|TurpGameplayAbility|TracetoFindTargets (Variables|Default|GetMouseHitLocation) true)
                  (Ability|EndAbility))))))))))

(event Ability|EventOnEndAbility
  (params (bWasCancelled :type Boolean)))