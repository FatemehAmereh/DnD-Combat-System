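; Bless gameplay ability that lets the player pick targets under the mouse and applies a gameplay effect to them.
; Target selection repeats, retrying invalid picks and adding valid ones to the GameState's combat packet until the target count is reached.
; It then calls face-target and plays a cast montage, whose Shoot AnimNotify event applies the effect to all targets.
; The ability ends when the montage completes.
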(event Ability|EventActivateAbility
  ;[1 1 1] Receive Targets
  (bind _targetdata (|GetTargetDataUnderMouse :!label _label)
    (:MouseTargetData
      (if (Utilities|IsValid (.ASC (Utilities|Struct|BreakTurpAbilityTargetData _targetdata)))
        (Class|TurpAbilitySystemBlueprintFL|AddTargetforCombatPacket (Variables|Default|GetTurpGameState) _targetdata)
        (Variables|Default|SetTargetsReceived (+ (Variables|Default|GetTargetsReceived) 1))
        (if (< (Variables|Default|GetTargetsReceived) (.TargetCount (Utilities|Struct|BreakGameplayAbilityProperties (Variables|Default|GetGameplayAbilityProperties))))
          (goto _label)
          (else
            (Class|TurpGameplayAbility|FaceTargetBeforeAttacking "0, 0, 0")
            (|PlayMontageandWaitProxy "None" "/Game/Assets/Animations/AM_MagicCastUp.AM_MagicCastUp" 1.0 "None" true 1.0 0.0 false
              (:then
                ;[1 0.3431 0.9228] Wait for AnimNotify on Montage
                (Ability|Tasks|WaitGameplayEvent "(TagName=\"AnimNotify.Shoot\")" 0 true
                  (:EventReceived
                    (Class|TurpAbilitySystemBlueprintFL|ApplyGameplayEffecttoAllTargets (Variables|Default|GetTurpGameState)))))
              (:OnCompleted
                (Ability|EndAbility)))))
        (else
          (goto _label))))))

(event Ability|EventOnEndAbility
  (params (bWasCancelled :type Boolean)))