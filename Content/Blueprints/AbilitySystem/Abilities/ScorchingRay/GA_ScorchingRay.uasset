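; Gameplay ability for Scorching Ray, a multi-target projectile spell aimed with the mouse.
; On activation it repeats an under-mouse targeting task, adding each pick to the game state's combat packet until the configured target count is reached.
; It then plays a magic attack montage and spawns projectiles on the Shoot anim notify gameplay event.
; The ability ends only from the montage's Completed pin.
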(event Ability|EventActivateAbility
  ;[1 1 1] Receive Targets
  (bind _targetdata (|GetTargetDataUnderMouse :!label _label)
    (:MouseTargetData
      (Class|TurpAbilitySystemBlueprintFL|AddTargetforCombatPacket (Variables|Default|GetTurpGameState) _targetdata)
      (bind _output_get (Variables|Default|SetTargetsReceived (+ (Variables|Default|GetTargetsReceived) 1)))
      (if (< _output_get (.TargetCount (Utilities|Struct|BreakGameplayAbilityProperties (Variables|Default|GetGameplayAbilityProperties))))
        (goto _label)
        (else
          (|PlayMontageandWaitProxy "None" "/Game/Assets/Animations/AM_MagicAttack02.AM_MagicAttack02" 1.0 "None" true 1.0 0.0 false
            (:then
              ;[1 0.3431 0.9228] Wait for AnimNotify on Montage
              (Ability|Tasks|WaitGameplayEvent "(TagName=\"AnimNotify.Shoot\")" 0 true
                (:EventReceived
                  (Class|ScorchingRay|SpawnProjectiles))))
            (:OnCompleted
              (Ability|EndAbility))))))))

(event Ability|EventOnEndAbility
  (params (bWasCancelled :type Boolean)))