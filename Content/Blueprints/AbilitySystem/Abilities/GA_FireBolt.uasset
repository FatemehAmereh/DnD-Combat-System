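; GA_FireBolt is a Fire Bolt gameplay ability that aims at the mouse cursor, with projectile spawning still a debug print placeholder.
; On activation it waits for mouse target data, then reads and debug-draws the first target location from the game state's CombatPacket.
; It plays a magic attack montage and waits once for the Events.Fire notify event to mark the spawn moment, ending when the montage completes.
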(event Ability|EventActivateAbility
  (Development|PrintString "FireBolt activated" true true "(R=0.000000,G=0.660000,B=1.000000,A=1.000000)" 1.0)
  (|GetTargetDataUnderMouse
    (:MouseTargetData
      (bind _output_get (Variables|Default|SetTargetLocation (Utilities|Array|Get(acopy) (.TargetLocations (Utilities|Struct|BreakCombatPacket (Variables|/Script/Turp.TurpGameStateBase|GetCombatPacket (Variables|Default|GetTurpGameState)))))))
      (Rendering|Debug|DrawDebugSphere _output_get 1e+02 12 "(R=1.000000,G=1.000000,B=1.000000,A=1.000000)" 5.0)
      (|PlayMontageandWaitProxy "None" "/Game/Characters/Mannequins/Animations/Quinn/AM_MagicAttack01.AM_MagicAttack01" 1.0 "None" true 1.0 0.0 false
        (:then
          ;[1 0.3431 0.9228] Wait for AnimNotify on Montage
          (Ability|Tasks|WaitGameplayEvent "(TagName=\"Events.Fire\")" 0 true
            (:EventReceived
              (Development|PrintString "Spawn projectile"))))
        (:OnCompleted
          (Ability|EndAbility))))))

(event Ability|EventOnEndAbility
  (params (bWasCancelled :type Boolean)))